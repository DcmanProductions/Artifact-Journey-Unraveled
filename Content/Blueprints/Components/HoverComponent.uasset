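; A hover component that keeps its owning actor floating above surfaces using physics forces.
; On BeginPlay it takes the owner's first primitive component and enables physics simulation on it.
; Each tick it traces downward from its own location and, on a hit, pushes that body along the surface normal with force fading linearly over trace distance.
; Linear and angular damping are applied on hits and never reset.
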(event EventBeginPlay
  ;[1 1 1] Begin Play
  (bind _output_get (Variables|Default|SetComponent (Utilities|Array|Get(acopy) (Actor|GetComponentsByClass (Components|GetOwner) "/Script/Engine.PrimitiveComponent"))))
  (Physics|SetSimulatePhysics _output_get true))

(event EventTick
  (params (DeltaSeconds :type Float%20%28single-precision%29))
  (bind _returnvalue (Transformation|GetWorldLocation))
  (bind _component (Variables|Default|GetComponent))
  ;[1 1 1] TIck
  (bind (_outhit _returnvalue_2) (Collision|LineTraceByChannel _returnvalue (- _returnvalue (Math|Vector|MakeVector 0.0 0.0 (Variables|Hover|GetTraceLength))) "TraceTypeQuery1" false 0 "None"))
  (if _returnvalue_2
    (Physics|AddForce _component (* (.ImpactNormal (Collision|BreakHitResult _outhit)) (Math|Float|Lerp (Variables|Hover|GetHoverForce) 0.0 (/ (Math|Vector|VectorLength (- (.Location (Collision|BreakHitResult _outhit)) (Transformation|GetWorldLocation))) (Variables|Hover|GetTraceLength)))) "None" false)
    (Class|PrimitiveComponent|SetLinearDamping _component (Variables|Hover|GetLinearDamping))
    (Class|PrimitiveComponent|SetAngularDamping _component (Variables|Hover|GetAngularDamping))))