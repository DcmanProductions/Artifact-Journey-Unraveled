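; Boss portal actor that stages the boss encounter intro and shuts its portal once the boss is dead.
; BeginPlay locks player input, launches the Artifact upward on a first encounter or removes it otherwise, then animates the portal open through timed flipbook swaps.
; It starts the Level1boss audio on a spawned AmbientSound, restores input and calls Spawn on BossToSpawn.
; Tick polls the boss's IsDead flag to switch the portal off.
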(event EventBeginPlay
  (Input|DisableInput (Game|GetPlayerCharacter 0) (Game|GetPlayerController 0))
  (if (Variables|Spawner|GetIsFirstEncounter)
    (Utilities|FlowControl|Delay 2.0)
    (Physics|AddForce (Variables|Default|GetArtifact) "0, 0,50000.000000" "None" true)
    (else
      (Components|DestroyComponent (Variables|Default|GetArtifact))
      (Utilities|FlowControl|Delay 2.0)))
  (Sprite|SetFlipbook (Variables|Default|GetPortal) "/Game/Animation/Level/PortalActivating.PortalActivating")
  (Utilities|FlowControl|Delay 0.11)
  (Sprite|SetFlipbook (Variables|Default|GetPortal) "/Game/Animation/Level/Portal_on.Portal_on")
  (bind _returnvalue (Game|SpawnActorfromClass "/Script/Engine.AmbientSound" (Math|Transform|MakeTransform "0, 0, 0" "0, 0, 0" "1,1,1") "Undefined" 0 0))
  (Audio|Components|Audio|SetSound (Variables|/Script/Engine.AmbientSound|GetAudioComponent _returnvalue) "/Game/Sound/Music/level1boss.level1boss")
  (Class|AudioComponent|SetUISound (Variables|/Script/Engine.AmbientSound|GetAudioComponent _returnvalue) true)
  (Audio|Components|Audio|Play (Variables|/Script/Engine.AmbientSound|GetAudioComponent _returnvalue) 0.0)
  (Utilities|FlowControl|Delay 0.7)
  (Input|EnableInput (Game|GetPlayerCharacter 0) (Game|GetPlayerController 0))
  (Default|Spawn (Variables|Spawner|GetBossToSpawn)))

(event EventTick
  (params (DeltaSeconds :type Float%20%28single-precision%29))
  (bind _bosstospawn (Variables|Spawner|GetBossToSpawn))
  (if (Utilities|IsValid _bosstospawn)
    (if (Variables|/Game/Blueprints/Entities/Enemies/Enemy.Enemy_C|GetIsDead _bosstospawn)
      (Sprite|SetFlipbook (Variables|Default|GetPortal) "/Game/Animation/Level/Portal_off.Portal_off"))))

(fn ConstructionScript)