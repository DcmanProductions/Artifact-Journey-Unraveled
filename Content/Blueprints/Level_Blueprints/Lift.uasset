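; Lift actor that shuttles endlessly between StartPosition and EndPosition actors, starting on BeginPlay and pausing for TimeSpentOnLevel at each end.
; Movement eases via VInterpTo in short Delay loops instead of Tick or a Timeline, with a Gate per direction.
; Arrival within a small tolerance closes the current Gate and, after the pause, starts the opposite leg.
; Overlapping its DeathBox kills Player and Enemy actors.
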(event OnComponentBeginOverlap(DeathBox)
  (params (OverlappedComponent :type Primitive%20Component%20Object%20Reference) (OtherActor :type Actor%20Object%20Reference) (OtherComp :type Primitive%20Component%20Object%20Reference) (OtherBodyIndex :type Integer) (bFromSweep :type Boolean) (SweepResult :type Hit%20Result%20Structure%20%28by%20ref%29))
  (bind _asplayer (Utilities|Casting|CastToPlayer OtherActor)
    (:then
      (Default|Death _asplayer))
    (:CastFailed
      (bind _asenemy (Utilities|Casting|CastToEnemy OtherActor))
      (Default|OnDeath _asenemy))))

(event EventBeginPlay
  (bind _returnvalue (Transformation|GetActorLocation))
  (bind _returnvalue_2 (Transformation|GetActorLocation))
  (bind _start_position (Variables|LiftComponent|GetStart%20Position))
  (bind _end_position (Variables|LiftComponent|GetEnd%20Position))
  (bind _returnvalue_3 (Transformation|GetActorLocation _start_position))
  (bind _returnvalue_4 (Transformation|GetActorLocation _end_position))
  (Utilities|FlowControl|Sequence :!label _label
    (:then_0
      (Transformation|SetActorLocation (Math|Interpolation|VInterpTo _returnvalue _returnvalue_4 (Utilities|Time|GetWorldDeltaSeconds) 2.0) false false :!label _label_2)
      (Utilities|FlowControl|Delay 0.01)
      (Utilities|FlowControl|Sequence
        (:then_0
          (Utilities|FlowControl|Gate true :!label _label_3
            (:Exit
              (goto _label_2))))
        (:then_1
          (if (Math|Vector|Equal(Vector) _returnvalue _returnvalue_4 3.0)
            (Utilities|FlowControl|Delay (Variables|LiftComponent|GetTimeSpentOnLevel))
            (Utilities|FlowControl|Sequence
              (:then_0
                (goto _label_3 Close))
              (:then_1
                (Utilities|FlowControl|Sequence
                  (:then_0
                    (Transformation|SetActorLocation (Math|Interpolation|VInterpTo _returnvalue_2 _returnvalue_3 (Utilities|Time|GetWorldDeltaSeconds) 2.0) false false :!label _label_4)
                    (Utilities|FlowControl|Delay 0.01)
                    (Utilities|FlowControl|Sequence
                      (:then_0
                        (Utilities|FlowControl|Gate true :!label _label_5
                          (:Exit
                            (goto _label_4))))
                      (:then_1
                        (if (Math|Vector|Equal(Vector) _returnvalue_2 _returnvalue_3 3.0)
                          (Utilities|FlowControl|Delay (Variables|LiftComponent|GetTimeSpentOnLevel))
                          (Utilities|FlowControl|Sequence
                            (:then_0
                              (goto _label_5 Close))
                            (:then_1
                              (goto _label)))))))
                  (:then_1
                    (goto _label_5 Open)))))))))
    (:then_1
      (goto _label_3 Open))))

(fn ConstructionScript)