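; Paper2D side-scroller player character with walk, sprint, double jump, light and dash attacks, health, shields, coins and lives.
; Tick picks flipbooks and facing from state flags, while damage adds knockback and brief invulnerability flags.
; BeginPlay restores stats from the PlayerPersistantData game instance, which teleports and death write back before level changes or respawn.
; It also creates the HUD, transition and pause widgets and applies saved sound settings.
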(event Custom|Dash%20Attack
  ;[1 1 1] Attacks
  (CallFunction|DashAttack))

(event Custom|UpdateAnimation
  (bind _returnvalue (Transformation|GetVelocity))
  (bind _returnvalue_2 (Math|Vector|VectorLength _returnvalue))
  (bind _returnvalue_3 (> _returnvalue_2 0.0))
  ;[1 1 1] Handle Animation
  (if (not (Variables|PlayerStats|GetBeingDamaged))
    (if (not (Variables|PlayerStats|GetDead))
      (if (AI|Components|NavMovement|IsFalling (Variables|Character|GetCharacterMovement))
        (Sprite|SetFlipbook (Variables|Default|GetSprite) "/Game/Animation/Entities/Character/Jump.Jump")
        (else
          (Variables|Movement|SetHasDoubleJumped false)
          (if (Variables|Movement|GetSprinting)
            (Sprite|SetFlipbook (Variables|Default|GetSprite) (select _returnvalue_3 "/Game/Animation/Entities/Character/Run.Run" "/Game/Animation/Entities/Character/idle.Idle"))
            (Variables|/Script/Engine.CharacterMovementComponent|SetMaxWalkSpeed (Variables|Character|GetCharacterMovement) (Variables|Movement|GetRunning%20Speed%20))
            (else
              (Sprite|SetFlipbook (Variables|Default|GetSprite) (select _returnvalue_3 "/Game/Animation/Entities/Character/Run.Run" "/Game/Animation/Entities/Character/idle.Idle"))
              (Variables|/Script/Engine.CharacterMovementComponent|SetMaxWalkSpeed (Variables|Character|GetCharacterMovement) (Variables|Movement|GetWalk%20Speed)))))))))

(event Custom|Damaged
  ;[1 1 1] Being Damaged Event
  (if (not (Variables|PlayerStats|GetDead))
    (Variables|PlayerStats|SetIsInvulnerable true)
    (if (not (Variables|PlayerStats|GetBeingDamaged))
      (Components|Movement|StopMovementImmediately (Variables|Character|GetCharacterMovement))
      (Variables|PlayerStats|SetBeingDamaged true)
      (Sprite|SetFlipbook (Variables|Default|GetSprite) "/Game/Animation/Entities/Character/Damaged.Damaged")
      (Character|LaunchCharacter (Math|Vector|SelectVector "-700.000000, 0,300.000000" "700.000000,0.000000,300.000000" (Variables|Movement|GetMovingRight)) true true)
      (Default|UpdateHearts (Variables|Widgets|GetHealthWidget))
      (Utilities|FlowControl|Delay 0.2)
      (Variables|PlayerStats|SetBeingDamaged false)
      (Utilities|FlowControl|Delay 0.2)
      (Variables|PlayerStats|SetIsInvulnerable false))))

(event Custom|Teleport
  (params (Level :type String) (IsInnerLevel :type Boolean) (InnerLevelLocation :type Vector))
  (bind _sprite (Variables|Default|GetSprite))
  ;[1 1 1] Teleporter
  (Variables|PlayerStats|SetTeleporting true)
  (bind _asplayer_persistant_data (Utilities|Casting|CastToPlayerPersistantData (Game|GetGameInstance)))
  (Variables|/Game/Blueprints/Managers/PlayerPersistantData.PlayerPersistantData_C|SetTimeMill _asplayer_persistant_data (Variables|Timer|GetTimeMill))
  (Variables|/Game/Blueprints/Managers/PlayerPersistantData.PlayerPersistantData_C|SetTimeSec _asplayer_persistant_data (Variables|Timer|GetTimeSec))
  (Variables|/Game/Blueprints/Managers/PlayerPersistantData.PlayerPersistantData_C|SetTimeMin _asplayer_persistant_data (Variables|Timer|GetTimeMin))
  (Variables|/Game/Blueprints/Managers/PlayerPersistantData.PlayerPersistantData_C|SetCurrentArtifactsPieces _asplayer_persistant_data (Variables|PlayerStats|GetArtifactsCollected))
  (Variables|/Game/Blueprints/Managers/PlayerPersistantData.PlayerPersistantData_C|SetCoins _asplayer_persistant_data (Variables|PlayerStats|GetCoins))
  (Variables|/Game/Blueprints/Managers/PlayerPersistantData.PlayerPersistantData_C|SetHealth _asplayer_persistant_data (Variables|PlayerStats|GetHealth))
  (Variables|/Game/Blueprints/Managers/PlayerPersistantData.PlayerPersistantData_C|SetLives _asplayer_persistant_data (Variables|PlayerStats|GetLives))
  (Variables|/Game/Blueprints/Managers/PlayerPersistantData.PlayerPersistantData_C|SetHasSuperPunch _asplayer_persistant_data (Variables|PlayerStats|GetHasSuperPunch))
  (Variables|/Game/Blueprints/Managers/PlayerPersistantData.PlayerPersistantData_C|SetShieldUnits _asplayer_persistant_data (Variables|PlayerStats|GetInvulnerability))
  (Components|Movement|StopMovementImmediately (Variables|Character|GetCharacterMovement))
  (Input|DisableInput 0)
  (Sprite|SetFlipbook _sprite "/Game/Animation/Entities/Character/Damaged.Damaged")
  (bind _returnvalue (Effects|SpawnEmitterAttached "/Game/ParticleSystem/Teleporting.Teleporting" _sprite "" "-10.000000, 0,-26.000000" "0,-90.000000, 0" "0.250000,0.250000,0.250000" "KeepRelativeOffset" false))
  (Audio|PlaySound2D "/Game/Sound/SFX/teleport.teleport" 1.0 1.0 0.0 0 0)
  (Utilities|FlowControl|Delay 2.0)
  (Default|OnLoadExit (Variables|Widgets|GetCurrentLoadLevelWidget))
  (Components|DestroyComponent _returnvalue)
  (Utilities|FlowControl|Delay 1.0)
  (if IsInnerLevel
    (Transformation|SetActorLocation InnerLevelLocation false true)
    (Utilities|FlowControl|Delay 0.2)
    (Default|OnLoadEnter (Variables|Widgets|GetCurrentLoadLevelWidget))
    (Input|EnableInput 0)
    (Sprite|SetFlipbook (Variables|Default|GetSprite) "/Game/Animation/Entities/Character/idle.Idle")
    (Variables|PlayerStats|SetTeleporting false)
    (else
      (Game|OpenLevel(byName) (Utilities|String|StringToName Level)))))

(event Custom|Death
  ;[1 1 1] On Death Event
  (if (not (Variables|PlayerStats|GetDead))
    (Variables|PlayerStats|SetDead true)
    (bind _asplayer_persistant_data (Utilities|Casting|CastToPlayerPersistantData (Game|GetGameInstance)))
    (Variables|/Game/Blueprints/Managers/PlayerPersistantData.PlayerPersistantData_C|SetTimeMill _asplayer_persistant_data (Variables|Timer|GetTimeMill))
    (Variables|/Game/Blueprints/Managers/PlayerPersistantData.PlayerPersistantData_C|SetTimeSec _asplayer_persistant_data (Variables|Timer|GetTimeSec))
    (Variables|/Game/Blueprints/Managers/PlayerPersistantData.PlayerPersistantData_C|SetTimeMin _asplayer_persistant_data (Variables|Timer|GetTimeMin))
    (Input|DisableInput 0)
    (Sprite|SetFlipbook (Variables|Default|GetSprite) "/Game/Animation/Entities/Character/Dying.Dying")
    (Utilities|FlowControl|Delay 0.4)
    (Sprite|SetFlipbook (Variables|Default|GetSprite) "/Game/Animation/Entities/Character/Dead.Dead")
    (Utilities|FlowControl|Delay 1.0)
    (Default|OnLoadExit (Variables|Widgets|GetCurrentLoadLevelWidget))
    (Utilities|FlowControl|Delay 1.0)
    (bind _asplayer_persistant_data_2 (Utilities|Casting|CastToPlayerPersistantData (Game|GetGameInstance))
      (:then
        (Variables|/Game/Blueprints/Managers/PlayerPersistantData.PlayerPersistantData_C|SetHasSuperPunch _asplayer_persistant_data_2 false)
        (Variables|/Game/Blueprints/Managers/PlayerPersistantData.PlayerPersistantData_C|SetShieldUnits _asplayer_persistant_data_2 0)
        (Variables|/Game/Blueprints/Managers/PlayerPersistantData.PlayerPersistantData_C|SetCoins _asplayer_persistant_data_2 (/ (Variables|PlayerStats|GetCoins) 3))
        (Variables|/Game/Blueprints/Managers/PlayerPersistantData.PlayerPersistantData_C|SetHealth _asplayer_persistant_data_2 4)
        (bind _result (Math|Integer|DecrementInt (Variables|PlayerStats|GetLives))
          (:%20%20
            (bind _output_get (Variables|/Game/Blueprints/Managers/PlayerPersistantData.PlayerPersistantData_C|SetLives _asplayer_persistant_data_2 _result))
            (Variables|/Game/Blueprints/Managers/PlayerPersistantData.PlayerPersistantData_C|SetCurrentArtifactsPieces _asplayer_persistant_data_2 (Variables|PlayerStats|GetArtifactsCollected))
            (Utilities|FlowControl|Delay 1.75)
            (if (< _output_get 0)
              (Game|OpenLevel(byName) "MainMenu" :!label _label)
              (else
                (bind _returnvalue (Game|GetCurrentLevelName true))
                (Game|OpenLevel(byName) (Utilities|String|StringToName _returnvalue)))))))
      (:CastFailed
        (goto _label)))))

(event Custom|Load%20and%20Apply%20Settings
  ;[1 1 1] Load Settings
  (bind (_master _music _sfx) (CallFunction|LoadSoundSettings))
  (CallFunction|ApplySoundSettings _master _music _sfx)
  (CallFunction|SaveSoundSettings _master _music _sfx)
  (bind _assave_sound_settings (Utilities|Casting|CastToSaveSoundSettings (Variables|Saves|GetSave%20Sound))))

(event Custom|Add%20Coins
  (params (Amount :type Integer))
  ;[1 1 1] Add Coins
  (bind _result (Math|Integer|IncrementInt (Variables|PlayerStats|GetCoins))
    (:%20%20
      (bind _output_get (Variables|PlayerStats|SetCoins _result))
      (bind _asplayer_persistant_data (Utilities|Casting|CastToPlayerPersistantData (Game|GetGameInstance)))
      (Variables|/Game/Blueprints/Managers/PlayerPersistantData.PlayerPersistantData_C|SetCoins _asplayer_persistant_data _output_get)
      (Default|AddCoins (Variables|Widgets|GetHealthWidget) Amount))))

(event Custom|Save%20to%20Persistant
  ;[1 1 1] Save
  (bind _asplayer_persistant_data (Utilities|Casting|CastToPlayerPersistantData (Game|GetGameInstance)))
  (Variables|/Game/Blueprints/Managers/PlayerPersistantData.PlayerPersistantData_C|SetCoins _asplayer_persistant_data (Variables|PlayerStats|GetCoins))
  (Variables|/Game/Blueprints/Managers/PlayerPersistantData.PlayerPersistantData_C|SetHealth _asplayer_persistant_data (Variables|PlayerStats|GetHealth))
  (Variables|/Game/Blueprints/Managers/PlayerPersistantData.PlayerPersistantData_C|SetLives _asplayer_persistant_data (Variables|PlayerStats|GetLives)))

(event Custom|Spurt%20Shot%20Attack
  ;[1 1 1] Attacks
  (if (not (AI|Components|NavMovement|IsFalling (Variables|Character|GetCharacterMovement)))
    (Variables|Movement|SetUsing%20Light%20Attack true)
    (Sprite|SetFlipbook (Variables|Default|GetSprite) "/Game/Animation/Entities/Character/Attacks/AttackA.AttackA")
    (Components|Movement|StopMovementImmediately (Variables|Character|GetCharacterMovement))
    (Utilities|FlowControl|Delay 0.5)
    (Variables|Movement|SetUsing%20Light%20Attack false)))

(event EventTick
  (params (DeltaSeconds :type Float%20%28single-precision%29))
  (bind _returnvalue (Pawn|GetController))
  (bind _returnvalue_2 (Pawn|GetController))
  ;[1 1 1] Tick - Updates animation
  (if (not (or (Variables|PlayerStats|GetTeleporting) (Variables|PlayerStats|GetDead)))
    (if (Variables|Movement|GetUsing%20Light%20Attack)
      (CallFunction|SpurtShotAttack)
      (Math|Float|CompareFloat (.X (Math|Vector|BreakVector (Variables|/Script/Engine.MovementComponent|GetVelocity (Pawn|GetMovementComponent)))) 0.0 :!label _label
        (:>
          (Utilities|IsValid _returnvalue_2 :!label _label_2
            (:Is%20Valid
              (Pawn|SetControlRotation _returnvalue_2 (Math|Rotator|MakeRotator 0.0 0.0 0.0)))))
        (:==
          (if (Variables|Movement|GetMovingRight)
            (goto _label_2)
            (else
              (Utilities|IsValid _returnvalue :!label _label_3
                (:Is%20Valid
                  (Pawn|SetControlRotation _returnvalue (Math|Rotator|MakeRotator 0.0 0.0 1.8e+02)))))))
        (:<
          (goto _label_3)))
      (elif (not (Variables|Movement|GetUsing%20Heavy%20Attack))
        (CallFunction|UpdateAnimation)
        (goto _label)))))

(event EventBeginPlay
  (bind _returnvalue (Game|GetPlayerController 0))
  (bind _healthwidget (Variables|Widgets|GetHealthWidget))
  ;[1 1 1] Begin Play
  (Class|ActorComponent|SetIsReplicated (Variables|Default|GetSprite) true)
  (CallFunction|SpawnHUD)
  (Variables|/Script/Engine.PlayerController|SetbShowMouseCursor _returnvalue false)
  (Input|SetInputModeGameOnly _returnvalue)
  (bind _returnvalue_2 (UserInterface|CreateWidget "/Game/Blueprints/UI/InGame/LoadLevelAnimation.LoadLevelAnimation_C"))
  (UserInterface|Viewport|AddtoViewport _returnvalue_2 0)
  (Default|OnLoadEnter _returnvalue_2)
  (Variables|Widgets|SetCurrentLoadLevelWidget _returnvalue_2)
  (CallFunction|LoadandApplySettings)
  (bind _asplayer_persistant_data (Utilities|Casting|CastToPlayerPersistantData (Game|GetGameInstance)))
  (Variables|PlayerStats|SetCurrentDifficulty (Variables|/Game/Blueprints/Managers/PlayerPersistantData.PlayerPersistantData_C|GetCurrentDifficulty _asplayer_persistant_data))
  (Variables|Timer|SetTimeMin (Variables|/Game/Blueprints/Managers/PlayerPersistantData.PlayerPersistantData_C|GetTimeMin _asplayer_persistant_data))
  (Variables|Timer|SetTimeMill (Variables|/Game/Blueprints/Managers/PlayerPersistantData.PlayerPersistantData_C|GetTimeMill _asplayer_persistant_data))
  (Variables|Timer|SetTimeSec (Variables|/Game/Blueprints/Managers/PlayerPersistantData.PlayerPersistantData_C|GetTimeSec _asplayer_persistant_data))
  (bind _returnvalue_3 (Game|GetCurrentLevelName true))
  (Variables|PlayerStats|SetArtifactsCollected (Variables|/Game/Blueprints/Managers/PlayerPersistantData.PlayerPersistantData_C|GetCurrentArtifactsPieces _asplayer_persistant_data))
  (Variables|/Game/Blueprints/Managers/PlayerPersistantData.PlayerPersistantData_C|SetLevelName _asplayer_persistant_data _returnvalue_3)
  (Variables|PlayerStats|SetLives (Variables|/Game/Blueprints/Managers/PlayerPersistantData.PlayerPersistantData_C|GetLives _asplayer_persistant_data))
  (Variables|PlayerStats|SetHealth (Variables|/Game/Blueprints/Managers/PlayerPersistantData.PlayerPersistantData_C|GetHealth _asplayer_persistant_data))
  (Variables|PlayerStats|SetCoins (Variables|/Game/Blueprints/Managers/PlayerPersistantData.PlayerPersistantData_C|GetCoins _asplayer_persistant_data))
  (bind _output_get (Variables|PlayerStats|SetHasSuperPunch (Variables|/Game/Blueprints/Managers/PlayerPersistantData.PlayerPersistantData_C|GetHasSuperPunch _asplayer_persistant_data)))
  (bind _output_get_2 (Variables|PlayerStats|SetInvulnerability (Variables|/Game/Blueprints/Managers/PlayerPersistantData.PlayerPersistantData_C|GetShieldUnits _asplayer_persistant_data)))
  (Default|UpdateHearts _healthwidget)
  (if (> _output_get_2 0)
    (Widget|SetRenderOpacity (Variables|/Game/Blueprints/UI/InGame/PlayerHUDWidget.PlayerHUDWidget_C|GetInvulnerabilitySection _healthwidget) 1.0))
  (if _output_get
    (Widget|SetRenderOpacity (Variables|/Game/Blueprints/UI/InGame/PlayerHUDWidget.PlayerHUDWidget_C|GetDamageEffectSection _healthwidget) 1.0)))

(event Input|ActionEvents|InputActionPause
  (params (Key :type Key%20Structure :default "None"))
  ;[1 1 1] Pause
  (:Pressed
    (CallFunction|Pause (not (Variables|PlayerStats|GetIsPaused)))))

(event Input|ActionEvents|InputActionSprint
  (params (Key :type Key%20Structure :default "None"))
  ;[1 1 1] Handle movement
  (:Pressed
    (Variables|Movement|SetSprinting true))
  (:Released
    (Variables|Movement|SetSprinting false)))

(event Input|ActionEvents|InputActionHeavyAttack
  (params (Key :type Key%20Structure :default "None"))
  ;[1 1 1] Handle Animation
  (:Pressed
    (if (not (Math|Boolean|ORBoolean (Variables|Movement|GetUsing%20Heavy%20Attack) (Variables|Movement|GetUsing%20Light%20Attack) (Variables|PlayerStats|GetDead)))
      (Variables|PlayerStats|SetIsInvulnerable true)
      (Variables|Movement|SetUsing%20Heavy%20Attack true)
      (CallFunction|DashAttack)
      (Utilities|FlowControl|Delay 0.25)
      (Variables|Movement|SetUsing%20Heavy%20Attack false)
      (Utilities|FlowControl|Delay 0.1)
      (Variables|PlayerStats|SetIsInvulnerable false))))

(event Input|ActionEvents|InputActionLightAttack
  (params (Key :type Key%20Structure :default "None"))
  ;[1 1 1] Handle Animation
  (:Pressed
    (if (not (Math|Boolean|ORBoolean (Variables|Movement|GetUsing%20Heavy%20Attack) (Variables|Movement|GetUsing%20Light%20Attack) (Variables|PlayerStats|GetDead)))
      (Variables|PlayerStats|SetIsInvulnerable true)
      (Variables|Movement|SetUsing%20Light%20Attack true)
      (Utilities|FlowControl|Delay 0.5)
      (Variables|Movement|SetUsing%20Light%20Attack false)
      (Utilities|FlowControl|Delay 0.1)
      (Variables|PlayerStats|SetIsInvulnerable false))))

(event Input|ActionEvents|InputActionJump
  (params (Key :type Key%20Structure :default "None"))
  (bind _hasdoublejumped (Variables|Movement|GetHasDoubleJumped))
  (bind _charactermovement (Variables|Character|GetCharacterMovement))
  (bind _returnvalue (AI|Components|NavMovement|IsFalling _charactermovement))
  ;[1 1 1] Handle Jump
  (:Pressed
    (if (and _returnvalue (not _hasdoublejumped))
      (CallFunction|DoubleJump)
      (Audio|PlaySound2D "/Game/Sound/SFX/playerjump.playerjump" 1.0 1.0 0.0 0 0)
      (else
        (Character|Jump)
        (if (not (and _hasdoublejumped _returnvalue))
          (Audio|PlaySound2D "/Game/Sound/SFX/playerjump.playerjump" 1.0 1.0 0.0 0 0)))))
  (:Released
    (Character|StopJumping)))

(event Input|AxisEvents|InputAxisMoveLeft
  (params (AxisValue :type Float%20%28single-precision%29))
  ;[1 1 1] Handle movement
  (if (not (Math|Boolean|ORBoolean (Variables|PlayerStats|GetDead) (Variables|PlayerStats|GetBeingDamaged) (Variables|PlayerStats|GetTeleporting)))
    (Pawn|Input|AddMovementInput "1.000000, 0,0.000000" AxisValue false)))

(event Input|AxisEvents|InputAxisMoveRight
  (params (AxisValue :type Float%20%28single-precision%29))
  ;[1 1 1] Handle movement
  (if (not (Math|Boolean|ORBoolean (Variables|PlayerStats|GetDead) (Variables|PlayerStats|GetBeingDamaged) (Variables|PlayerStats|GetTeleporting)))
    (Variables|Movement|SetMovingRight (> AxisValue 0.0))
    (Pawn|Input|AddMovementInput "1.000000, 0,0.000000" AxisValue false)))

(event Input|TouchEvents|InputTouch
  (params (Location :type Vector) (FingerIndex :type ETouchIndex%20Enum))
  (bind _hasdoublejumped (Variables|Movement|GetHasDoubleJumped))
  (bind _charactermovement (Variables|Character|GetCharacterMovement))
  (bind _returnvalue (AI|Components|NavMovement|IsFalling _charactermovement))
  ;[1 1 1] Handle Jump
  (:Pressed
    (if (and _returnvalue (not _hasdoublejumped))
      (CallFunction|DoubleJump)
      (Audio|PlaySound2D "/Game/Sound/SFX/playerjump.playerjump" 1.0 1.0 0.0 0 0)
      (else
        (Character|Jump)
        (if (not (and _hasdoublejumped _returnvalue))
          (Audio|PlaySound2D "/Game/Sound/SFX/playerjump.playerjump" 1.0 1.0 0.0 0 0)))))
  (:Released
    (Character|StopJumping)))

(fn ConstructionScript)

(fn DashAttack
  (Sprite|SetFlipbook (Variables|Default|GetSprite) "/Game/Animation/Entities/Character/Attacks/AttackD.AttackD")
  (if (Variables|Movement|GetMovingRight)
    (Character|LaunchCharacter (Math|Vector|MakeVector (Variables|Movement|GetDash%20Force) 0.0 0.0) true false)
    (else
      (Character|LaunchCharacter (Math|Vector|MakeVector (* (Variables|Movement|GetDash%20Force) -1.0) 0.0 0.0) true false)))
  (Audio|PlaySound2D "/Game/Sound/SFX/playercharge.playercharge" 1.0 1.0 0.0 0 0))

(fn DoubleJump
  (Character|LaunchCharacter "0,0.000000,750.000000" false true)
  (Variables|Movement|SetHasDoubleJumped true))

(fn Heal
  (params (Amount :type Integer))
  (Variables|PlayerStats|SetHealth (+ Amount (Variables|PlayerStats|GetHealth)))
  (Default|UpdateHearts (Variables|Widgets|GetHealthWidget)))

(fn Damage
  (params (Amount :type Integer))
  (if (> (Variables|PlayerStats|GetInvulnerability) 0)
    (bind _result (Math|Integer|DecrementInt (Variables|PlayerStats|GetInvulnerability))
      (:%20%20
        (if (< _result 0)
          (Variables|PlayerStats|SetInvulnerability 0))
        (if (== _result 0)
          (Widget|SetRenderOpacity (Variables|/Game/Blueprints/UI/InGame/PlayerHUDWidget.PlayerHUDWidget_C|GetInvulnerabilitySection (Variables|Widgets|GetHealthWidget)) 0.0))))
    (elif (< (- (Variables|PlayerStats|GetHealth) Amount) 0)
      (CallFunction|Damaged)
      (CallFunction|Death)
      (else
        (Variables|PlayerStats|SetHealth (- (Variables|PlayerStats|GetHealth) Amount))
        (CallFunction|Damaged)))))

(fn SpawnHUD
  (bind _returnvalue (UserInterface|CreateWidget "/Game/Blueprints/UI/InGame/PlayerHUDWidget.PlayerHUDWidget_C"))
  (UserInterface|Viewport|AddtoViewport _returnvalue 0)
  (Variables|Widgets|SetHealthWidget _returnvalue))

(fn Pause
  (params (Pause :type Boolean))
  (bind _returnvalue (Game|GetPlayerController 0))
  (bind _output_get (Variables|PlayerStats|SetIsPaused Pause))
  (bind _output_get_2 (Variables|/Script/Engine.PlayerController|SetbShowMouseCursor (Game|GetPlayerController 0) _output_get))
  (Game|SetGamePaused _output_get_2)
  (if _output_get_2
    (bind _returnvalue_2 (UserInterface|CreateWidget "/Game/Blueprints/UI/Menus/PauseMenu.PauseMenu_C"))
    (bind _output_get_3 (Variables|Widgets|SetPause%20Menu _returnvalue_2))
    (UserInterface|Viewport|AddtoViewport _output_get_3 0)
    (Input|SetInputModeUIOnly _returnvalue _output_get_3 "LockInFullscreen")
    (else
      (Widget|RemovefromParent (Variables|Widgets|GetPause%20Menu))
      (Input|SetInputModeGameOnly _returnvalue))))

(fn SaveSoundSettings
  (params (Master :type Float%20%28single-precision%29) (Music :type Float%20%28single-precision%29) (SFX :type Float%20%28single-precision%29))
  (bind _returnvalue (SaveGame|CreateSaveGameObject "/Game/Blueprints/GameData/SaveSoundSettings.SaveSoundSettings_C"))
  (bind _output_get (Variables|Saves|SetSave%20Sound _returnvalue))
  (bind _assave_sound_settings (Utilities|Casting|CastToSaveSoundSettings _output_get))
  (Variables|/Game/Blueprints/GameData/SaveSoundSettings.SaveSoundSettings_C|SetMaster _assave_sound_settings Master)
  (Variables|/Game/Blueprints/GameData/SaveSoundSettings.SaveSoundSettings_C|SetMusic _assave_sound_settings Music)
  (Variables|/Game/Blueprints/GameData/SaveSoundSettings.SaveSoundSettings_C|SetSFX _assave_sound_settings SFX)
  (SaveGame|SaveGametoSlot _returnvalue (Variables|Saves|GetSoundSettingSlotName)))

(fn LoadSoundSettings
  (bind _returnvalue (SaveGame|DoesSaveGameExist (Variables|Saves|GetSoundSettingSlotName)))
  (if _returnvalue
    (bind _returnvalue_2 (SaveGame|LoadGamefromSlot (Variables|Saves|GetSoundSettingSlotName)))
    (bind _output_get (Variables|Saves|SetSave%20Sound _returnvalue_2))
    (bind _assave_sound_settings (Utilities|Casting|CastToSaveSoundSettings _output_get))
    (return (Variables|/Game/Blueprints/GameData/SaveSoundSettings.SaveSoundSettings_C|GetMaster _assave_sound_settings) (Variables|/Game/Blueprints/GameData/SaveSoundSettings.SaveSoundSettings_C|GetMusic _assave_sound_settings) (Variables|/Game/Blueprints/GameData/SaveSoundSettings.SaveSoundSettings_C|GetSFX _assave_sound_settings))
    (else
      (return 1.0 1.0 1.0))))

(fn ApplySoundSettings
  (params (Master :type Float%20%28single-precision%29) (Music :type Float%20%28single-precision%29) (SFX :type Float%20%28single-precision%29))
  (Class|GameplayStatics|SetBaseSoundMix "/Game/Sound/Mixer.Mixer")
  (Audio|SetSoundMixClassOverride "/Game/Sound/Mixer.Mixer" "/Game/Sound/Master.Master" Master 1.0 0.0 true)
  (Audio|SetSoundMixClassOverride "/Game/Sound/Mixer.Mixer" "/Game/Sound/Music.Music" Music 1.0 0.0 true)
  (Audio|SetSoundMixClassOverride "/Game/Sound/Mixer.Mixer" "/Game/Sound/SFX.SFX" SFX 1.0 0.0 true))